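; Gate Blueprint that drives a linked Twin gate, flipping its activation state and animating it up or down.
; ToggleActivation swaps collision between GateBox, solid when activated, and DetectionBox, enabled when deactivated.
; Sync_Gate and BeginPlay both toggle the Twin, then play separate timelines that raise its Gate when activated or lower it otherwise.
; Timeline values offset the current relative Z on every update, so movement accumulates rather than interpolating between fixed endpoints.
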(event Custom|Sync_Gate
  (CallFunction|ToggleActivation (Variables|Default|GetTwin))
  (if (Variables|Gate_BP_C|GetIs%20Activated (Variables|Default|GetTwin))
    (bind _moveup (Timeline|AnimUp PlayFromStart)
      (:Update
        (Transformation|SetRelativeLocation (Variables|Gate_BP_C|GetGate (Variables|Default|GetTwin)) (Math|Vector|MakeVector 0.0 0.0 (+ _moveup (.z (Variables|/Script/Engine.SceneComponent|GetRelativeLocation (Variables|Gate_BP_C|GetGate (Variables|Default|GetTwin)))))) false false)))
    (else
      (bind _movedown (Timeline|AnimDown PlayFromStart)
        (:Update
          (Transformation|SetRelativeLocation (Variables|Gate_BP_C|GetGate (Variables|Default|GetTwin)) (Math|Vector|MakeVector 0.0 0.0 (- (.z (Variables|/Script/Engine.SceneComponent|GetRelativeLocation (Variables|Gate_BP_C|GetGate (Variables|Default|GetTwin)))) _movedown)) false false))))))

(event EventBeginPlay
  (CallFunction|ToggleActivation (Variables|Default|GetTwin))
  (if (Variables|Gate_BP_C|GetIs%20Activated (Variables|Default|GetTwin))
    (bind _moveup (Timeline|Timeline_2 PlayFromStart)
      (:Update
        (Transformation|SetRelativeLocation (Variables|Gate_BP_C|GetGate (Variables|Default|GetTwin)) (Math|Vector|MakeVector 0.0 0.0 (+ _moveup (.z (Variables|/Script/Engine.SceneComponent|GetRelativeLocation (Variables|Gate_BP_C|GetGate (Variables|Default|GetTwin)))))) false false)))
    (else
      (bind _movedown (Timeline|Timeline_3 PlayFromStart)
        (:Update
          (Transformation|SetRelativeLocation (Variables|Gate_BP_C|GetGate (Variables|Default|GetTwin)) (Math|Vector|MakeVector 0.0 0.0 (- (.z (Variables|/Script/Engine.SceneComponent|GetRelativeLocation (Variables|Gate_BP_C|GetGate (Variables|Default|GetTwin)))) _movedown)) false false))))))

(fn ConstructionScript)

(fn ToggleActivation
  (if (Variables|Default|GetIs%20Activated)
    (Variables|Default|SetIs%20Activated false)
    (Collision|SetCollisionEnabled (Variables|Default|GetGate_Box) "NoCollision")
    (Collision|SetCollisionEnabled (Variables|Default|GetDetectionBox) "QueryAndPhysics")
    (else
      (Variables|Default|SetIs%20Activated true)
      (Collision|SetCollisionEnabled (Variables|Default|GetGate_Box) "QueryAndPhysics")
      (Collision|SetCollisionEnabled (Variables|Default|GetDetectionBox) "NoCollision"))))